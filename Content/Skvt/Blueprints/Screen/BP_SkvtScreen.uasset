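; BP_SkvtScreen is a screen actor that displays a WBP_SkvtWeb widget through its Webpage component and can be switched on, switched off or destroyed.
; On BeginPlay it caches a reference to the web widget, while the Turnon and TurnOff events toggle the component's visibility.
; Destroy activates smoke and explosion effects, hides the page and sets IsDestroyed, which blocks all further toggling or repeat destruction.
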(event `self.ReceiveBeginPlay`
  (`self.Initialize`))

(event `/Game/Skvt/Blueprints/BPI_Electric.TurnOff`
  (if (not (`self.isDestroyed`))
    (`self.ToggleOn` false)))

(event `/Game/Skvt/Blueprints/BPI_Electric.TurnOn`
  (if (not (`self.isDestroyed`))
    (`self.ToggleOn` true)))

(event `/Game/Skvt/Blueprints/BPI_Electric.Destroy`
  (if (not (`self.isDestroyed`))
    (`ActorComponent.Activate` (`self.P_Smoke`) false)
    (`ActorComponent.Activate` (`self.P_Explosion`) false)
    (`self.ToggleOn` false)
    (set `self.isDestroyed` true)))

(fn `Initialize`
  (bind _aswbp_skvt_web (cast `/Game/Skvt/Blueprints/Screen/WBP_SkvtWeb` (`WidgetComponent.GetWidget` (`self.Webpage`))))
  (set `self.WebpageRef` _aswbp_skvt_web))

(fn `ToggleOn`
  (params (TurnOn :type Boolean))
  (`SceneComponent.SetVisibility` (`self.Webpage`) TurnOn false))

(fn `UserConstructionScript`)