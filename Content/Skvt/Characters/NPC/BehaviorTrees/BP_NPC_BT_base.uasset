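; Base NPC character Blueprint that jumps to a nav link point when the NavLinkinRange event fires.
; It computes a ballistic launch velocity from its location to that point, using math expressions based on JumpDuration and Gravity.
; LaunchCharacter applies the result with XY and Z override, replacing current velocity.
; BeginPlay, Tick and overlap events are disabled stubs, and the file contains no behavior tree logic.
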(event EventBeginPlay
  (|CallParentFunction) ; This node is disabled and will not be called.\nDrag off pins to build functionality.
)

(event Collision|EventActorBeginOverlap
  (params (OtherActor :type Actor%20Object%20Reference))
  (|CallParentFunction OtherActor) ; This node is disabled and will not be called.\nDrag off pins to build functionality.
)

(event EventTick
  (params (DeltaSeconds :type Float%20%28single-precision%29))
  (|CallParentFunction DeltaSeconds) ; This node is disabled and will not be called.\nDrag off pins to build functionality.
)

(event EventNavLinkinRange
  (params (NavLink :type Vector :default "0, 0, 0"))
  (bind (_x _y _z) (Math|Vector|BreakVector NavLink))
  (bind _returnvalue (Transformation|GetActorLocation))
  (bind (_x_2 _y_2 _z_2) (Math|Vector|BreakVector _returnvalue))
  (Character|LaunchCharacter (Math|Vector|MakeVector (|((DestinationX-StartX)/{B90C981E-43BE-2169-82DE-269802034D67}) _x _x_2) (|((DestinationY-StartY)/{B90C981E-43BE-2169-82DE-269802034D67}) _y _y_2) (|((DestinationHeight-(StartHeight-(((Power({B90C981E-43BE-2169-82DE-269802034D67},2))*0.500000)*{FBB7A915-47A6-7108-40E4-2486EEDA8F72})))/{B90C981E-43BE-2169-82DE-269802034D67}) _z _z_2)) true true))

(fn ConstructionScript
  (|CallParentFunction))